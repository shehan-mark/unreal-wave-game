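; WaveGamePlayerController_BP is a player controller Blueprint whose BeginPlay, Tick and construction script are all empty.
; Its only logic is a pause-menu toggle that is not connected to any event, so it never runs.
; That orphaned chain prints a debug string, then either creates a TESTWIDGET menu and pauses the game, or removes the menu and unpauses.
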(event EventBeginPlay)

(event EventTick
  (params (DeltaSeconds :type Float%20%28single-precision%29)))

(event Input|KeyboardEvents|O
  (params (Key :type Key%20Structure :default "None")))

(event Input|KeyboardEvents|Pause
  (params (Key :type Key%20Structure :default "None")))

(fn ConstructionScript)